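; Procedural map generator that builds a room layout at BeginPlay from a main room, cells at its Celdas points and random rooms at exit points.
; Each new room waits briefly for an overlap check, then is either destroyed and retried or adds its exits to the pool.
; A looping timer opens FirstPersonMap if generation outlasts a time limit equal to the initial room count in seconds.
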(event Custom|Spawn%20Main%20Room
  ;[0.02459 0.15 0.02609 0.5] Main Room
  (bind _returnvalue (Game|SpawnActorfromClass "/Game/ProceduralMap/BP_MasterRoom.BP_MasterRoom_C" (Transformation|GetWorldTransform (Variables|Default|GetDefaultSceneRoot)) "AlwaysSpawn" "MultiplyWithRoot" 0 0))
  (Utilities|Array|AppendArray (Variables|Default|GetCeldas%20List) (Components|GetChildrenComponents (Variables|/Game/ProceduralMap/BP_MasterRoom.BP_MasterRoom_C|GetCeldas _returnvalue) false))
  (Utilities|Array|AppendArray (Variables|Default|GetExits%20List) (Components|GetChildrenComponents (Variables|/Game/ProceduralMap/BP_MasterRoom.BP_MasterRoom_C|GetExits _returnvalue) false)))

(event Custom|Spawn%20Celdas
  ;[0.02459 0.15 0.02609 0.5] Celdas
  (bind _output_get (Variables|Default|SetSelected%20Celda (Utilities|Array|Get(acopy) (Variables|Default|GetCeldas%20List) (- (Variables|Default|GetCeldasCount) 1))))
  (Utilities|Array|RemoveItem (Variables|Default|GetCeldas%20List) _output_get)
  (bind _returnvalue (Game|SpawnActorfromClass (.OutItem (Utilities|Array|Random (Variables|Default|GetAvailable%20Celdas%20List))) (Transformation|GetWorldTransform _output_get) "AlwaysSpawn" "MultiplyWithRoot" 0 0))
  (Utilities|Casting|CastToBP_MasterRoom _returnvalue)
  (Variables|Default|SetCeldasCount (- (Variables|Default|GetCeldasCount) 1))
  (if (> (Variables|Default|GetCeldasCount) 0)
    (CallFunction|SpawnCeldas)))

(event Custom|Spawn%20Rooms
  ;[0.02459 0.15 0.02609 0.5] Rooms
  (Variables|Default|SetSelected%20Exit%20Point (.OutItem (Utilities|Array|Random (Variables|Default|GetExits%20List))))
  (bind _returnvalue (Game|SpawnActorfromClass (.OutItem (Utilities|Array|Random (Variables|Default|GetAvailable%20Room%20List))) (Transformation|GetWorldTransform (Variables|Default|GetSelected%20Exit%20Point)) "AlwaysSpawn" "MultiplyWithRoot" 0 0))
  (bind _asbp_master_room (Utilities|Casting|CastToBP_MasterRoom _returnvalue))
  (Variables|Default|SetLastest%20Room _asbp_master_room)
  (Utilities|FlowControl|Delay 0.1)
  (CallFunction|CheckOverlap))

(event Custom|Overlaping
  ;[0.02459 0.15 0.02609 0.5] Overlap Loop
  (for _array_element (Components|GetChildrenComponents (Variables|/Game/ProceduralMap/BP_MasterRoom.BP_MasterRoom_C|GetOverlap%20folder (Variables|Default|GetLastest%20Room)) false)
    (bind _asbox_collision (Utilities|Casting|CastToBoxComponent _array_element))
    (Utilities|Array|AppendArray (Variables|Default|GetOverlapped%20List) (Class|PrimitiveComponent|GetOverlappingComponents _asbox_collision))))

(event Custom|Start%20Map%20timer
  ;[0.03638 0.15 0.03923 0.5] Map timmer
  (bind _returnvalue (Utilities|Time|SetTimerbyEvent (delegate Custom|Check%20for%20Complete) 1.0 true))
  (Variables|Default|SetTimer%20Handle _returnvalue))

(event Custom|Check%20Overlap
  ;[0.02459 0.15 0.02609 0.5] Check Overlap
  (CallFunction|Overlaping)
  (if (Utilities|Array|IsNotEmpty (Variables|Default|GetOverlapped%20List))
    (Utilities|Array|Clear (Variables|Default|GetOverlapped%20List))
    (Actor|DestroyActor (Variables|Default|GetLastest%20Room))
    (CallFunction|SpawnRooms)
    (else
      (Utilities|Array|Clear (Variables|Default|GetOverlapped%20List))
      (Variables|Default|SetRoomsCount (- (Variables|Default|GetRoomsCount) 1))
      (Utilities|Array|AppendArray (Variables|Default|GetExits%20List) (Components|GetChildrenComponents (Variables|/Game/ProceduralMap/BP_MasterRoom.BP_MasterRoom_C|GetExits (Variables|Default|GetLastest%20Room)) false))
      (if (> (Variables|Default|GetRoomsCount) 0)
        (CallFunction|SpawnRooms)
        (else
          (Variables|Default|SetCompleteMap true)
          (Utilities|Time|ClearandInvalidateTimerbyHandle (Variables|Default|GetTimer%20Handle))
          (Development|PrintString "Spawning..." true false "(R=0.997333,G=1.000000,B=0.953415,A=1.000000)" 1e+01))))))

(event Custom|Check%20for%20Complete
  ;[0.03638 0.15 0.03923 0.5] Map timmer
  (Development|PrintString (Utilities|String|ToString(Integer) (Variables|Default|GetMax%20Map%20Timer)))
  (if (>= (Utilities|Time|GetGameTimeinSeconds) (Variables|Default|GetMax%20Map%20Timer))
    (Game|OpenLevel(byName) "FirstPersonMap")))

(event EventBeginPlay
  (CallFunction|SpawnMainRoom)
  (CallFunction|SpawnCeldas)
  (Variables|Default|SetMax%20Map%20Timer (Variables|Default|GetRoomsCount))
  (CallFunction|StartMapTimer)
  (CallFunction|SpawnRooms))

(event Collision|EventActorBeginOverlap
  (params (OtherActor :type Actor%20Object%20Reference)))

(event EventTick
  (params (DeltaSeconds :type Float%20%28single-precision%29)))

(fn ConstructionScript)